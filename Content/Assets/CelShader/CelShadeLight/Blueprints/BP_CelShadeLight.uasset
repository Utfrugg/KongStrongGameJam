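; BP_CelShadeLight is a placeable cel-shading light of shadow, directional, point, spot or area type.
; Every tick it writes its direction, location, type and color/falloff settings into two Material Parameter Collections, using channel-indexed parameter names.
; Initialization scans all such lights, clears unused or disabled slots among sixteen channels, and toggles the film tonemapper via console command.
; Construction also sets the type icon, arrow and channel label.
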(event `self.ReceiveBeginPlay`
  (`self.InitializeLight`))

(event `self.ReceiveTick`
  (params (DeltaSeconds :type "Float (single-precision)"))
  (`self.UpdateLight`))

(event `UpdateLight`
  (bind _lightchannel (`self.LightChannel`))
  (bind _lightchannel_2 (`self.LightChannel`))
  (bind _returnvalue (`KismetStringLibrary.Conv_IntToString` (+ _lightchannel_2 16)))
  (bind _returnvalue_2 (select `bool` (== _lightchannel_2 0) :`false` (`KismetStringLibrary.Conv_IntToString` _lightchannel_2)))
  (bind _returnvalue_3 (`KismetStringLibrary.Conv_StringToName` (`KismetStringLibrary.Concat_StrStr` "Scalar" _returnvalue_2)))
  (bind _returnvalue_4 (`KismetStringLibrary.Conv_StringToName` (`KismetStringLibrary.Concat_StrStr` "Vector" _returnvalue_2)))
  (`TextRenderComponent.K2_SetText` (`self.ChannelIndicator`) (`KismetTextLibrary.Conv_IntToText` (`self.LightChannel`) false false) :!label _label)
  (if (`self.Enable Light`)
    (`KismetMaterialLibrary.SetVectorParameterValue` "/Game/CelShader/CelShadeLight/ParameterCollections/MPC_LightTypeAngleLocation.MPC_LightTypeAngleLocation" _returnvalue_4 (`KismetMathLibrary.Conv_VectorToLinearColor` (`KismetMathLibrary.GetForwardVector` (`self.K2_GetActorRotation`))))
    (`KismetMaterialLibrary.SetVectorParameterValue` "/Game/CelShader/CelShadeLight/ParameterCollections/MPC_LightTypeAngleLocation.MPC_LightTypeAngleLocation" (`KismetStringLibrary.Conv_StringToName` (`KismetStringLibrary.Concat_StrStr` "Vector" _returnvalue)) (`KismetMathLibrary.Conv_VectorToLinearColor` (`self.K2_GetActorLocation`)))
    (`KismetMaterialLibrary.SetScalarParameterValue` "/Game/CelShader/CelShadeLight/ParameterCollections/MPC_LightTypeAngleLocation.MPC_LightTypeAngleLocation" _returnvalue_3 (select `/Game/CelShader/CelShadeLight/Enum/E_LightTypes` (`self.LightType`) :`NewEnumerator4` -1.0 :`NewEnumerator1` 1.0 :`NewEnumerator2` 2.0 :`NewEnumerator3` -2.0 :!type "Float (single-precision)"))
    (`KismetMaterialLibrary.SetScalarParameterValue` "/Game/CelShader/CelShadeLight/ParameterCollections/MPC_LightTypeAngleLocation.MPC_LightTypeAngleLocation" (`KismetStringLibrary.Conv_StringToName` (`KismetStringLibrary.Concat_StrStr` "Scalar" _returnvalue)) (`KismetMathLibrary.MapRangeClamped` (`self.SpotlightAngle`) 0.0 360.0 1.0 -1.0))
    (`KismetMaterialLibrary.SetVectorParameterValue` "/Game/CelShader/CelShadeLight/ParameterCollections/MPC_LightIntensityFalloffColor.MPC_LightIntensityFalloffColor" _returnvalue_4 (`KismetMathLibrary.Conv_ColorToLinearColor` (`self.Color`)))
    (`KismetMaterialLibrary.SetScalarParameterValue` "/Game/CelShader/CelShadeLight/ParameterCollections/MPC_LightIntensityFalloffColor.MPC_LightIntensityFalloffColor" _returnvalue_3 (`self.Intensity`))
    (`KismetMaterialLibrary.SetScalarParameterValue` "/Game/CelShader/CelShadeLight/ParameterCollections/MPC_LightIntensityFalloffColor.MPC_LightIntensityFalloffColor" (`KismetStringLibrary.Conv_StringToName` (`KismetStringLibrary.Concat_StrStr` "Scalar" (`KismetStringLibrary.Conv_IntToString` (+ _lightchannel 16)))) (`self.FullStrengthDistance`))
    (`KismetMaterialLibrary.SetScalarParameterValue` "/Game/CelShader/CelShadeLight/ParameterCollections/MPC_LightIntensityFalloffColor.MPC_LightIntensityFalloffColor" (`KismetStringLibrary.Conv_StringToName` (`KismetStringLibrary.Concat_StrStr` "Scalar" (`KismetStringLibrary.Conv_IntToString` (+ _lightchannel 32)))) (`self.FalloffDistance`))
    (set `ArrowComponent.ArrowColor` (`self.Color`) (`self.Arrow`))))

(event `InitializeLight`
  (`self.ResetLights`)
  (goto _label))

(event `ResetLights`
  (bind _activechannels (`self.ActiveChannels`))
  (`KismetArrayLibrary.Array_Clear` (`self.ActiveChannels`))
  (bind _outactors (`GameplayStatics.GetAllActorsOfClass` "BP_CelShadeLight_C"))
  (for _array_element _outactors
    (`KismetArrayLibrary.Array_Add` _activechannels (`/Game/Assets/CelShader/CelShadeLight/Blueprints/BP_CelShadeLight.LightChannel` _array_element))
    (if (and (!= _array_element self) (`self.RefreshLights`))
      (`self.InitializeLight` _array_element)))
  (set `self.RefreshLights` false)
  (for _index (range 16)
    (if (`KismetArrayLibrary.Array_Contains` _activechannels _index)
      (if (and (== _index (`self.LightChannel`)) (not (`self.Enable Light`)))
        (bind _returnvalue (select `bool` (== _index 0) :`false` (`KismetStringLibrary.Conv_IntToString` _index)))
        (`KismetMaterialLibrary.SetVectorParameterValue` "/Game/CelShader/CelShadeLight/ParameterCollections/MPC_LightTypeAngleLocation.MPC_LightTypeAngleLocation" (`KismetStringLibrary.Conv_StringToName` (`KismetStringLibrary.Concat_StrStr` "Vector" _returnvalue)) (make `LinearColor` 0.0) :!label _label_2)
        (`KismetMaterialLibrary.SetVectorParameterValue` "/Game/CelShader/CelShadeLight/ParameterCollections/MPC_LightTypeAngleLocation.MPC_LightTypeAngleLocation" (`KismetStringLibrary.Conv_StringToName` (`KismetStringLibrary.Concat_StrStr` "Vector" (`KismetStringLibrary.Conv_IntToString` (+ _index 16)))) (make `LinearColor` 0.0))
        (`KismetMaterialLibrary.SetScalarParameterValue` "/Game/CelShader/CelShadeLight/ParameterCollections/MPC_LightTypeAngleLocation.MPC_LightTypeAngleLocation" (`KismetStringLibrary.Conv_StringToName` (`KismetStringLibrary.Concat_StrStr` "Scalar" _returnvalue))))
      (else
        (goto _label_2))))
  (set `self.TonemapperIsDisabled` false)
  (for _array_element_2 _outactors
    (if (`/Game/Assets/CelShader/CelShadeLight/Blueprints/BP_CelShadeLight.DisableFilmTonemapper` _array_element_2)
      (`KismetSystemLibrary.ExecuteConsoleCommand` "r.TonemapperFilm 0" null)
      (set `self.TonemapperIsDisabled` true)))
  (if (not (`self.TonemapperIsDisabled`))
    (`KismetSystemLibrary.ExecuteConsoleCommand` "r.TonemapperFilm 1" null)))

(fn `UserConstructionScript`
  (bind _channelindicator (`self.ChannelIndicator`))
  (bind _lighttype (`self.LightType`))
  (bind _arrow (`self.Arrow`))
  (bind _returnvalue (select `/Game/CelShader/CelShadeLight/Enum/E_LightTypes` _lighttype :`NewEnumerator0` true :`NewEnumerator2` true))
  (`self.InitializeLight`)
  (set `SceneComponent.bAbsoluteRotation` true _channelindicator)
  (`SceneComponent.K2_SetWorldLocationAndRotation` :`self` _channelindicator :`NewLocation` (+ (`self.K2_GetActorLocation`) (0.0 -25.0 -30.0)))
  (`BillboardComponent.SetSprite` (`self.Billboard`) (select `/Game/CelShader/CelShadeLight/Enum/E_LightTypes` _lighttype :`NewEnumerator4` "/Game/CelShader/CelShadeLight/Icons/T_CelIconShadow_D.T_CelIconShadow_D" :`NewEnumerator0` "/Game/CelShader/CelShadeLight/Icons/T_CelIconDirectional_D.T_CelIconDirectional_D" :`NewEnumerator1` "/Game/CelShader/CelShadeLight/Icons/T_CelIconPoint_D.T_CelIconPoint_D" :`NewEnumerator2` "/Game/CelShader/CelShadeLight/Icons/T_CelIconSpot_D.T_CelIconSpot_D" :`NewEnumerator3` "/Game/CelShader/CelShadeLight/Icons/T_CelIconArea_D.T_CelIconArea_D" :!type "Texture2D Object Reference"))
  (`SceneComponent.SetVisibility` _arrow _returnvalue false)
  (`SceneComponent.SetHiddenInGame` _arrow (not _returnvalue) false))