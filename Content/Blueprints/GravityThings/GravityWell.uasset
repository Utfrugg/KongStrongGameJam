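; GravityWell is an actor that applies a radial force to its surroundings, built on a RadialForce component.
; On BeginPlay it copies its Falloff and ForceStrength variables onto that component.
; While Enabled is true, it calls FireImpulse on the component every Tick, producing repeated impulses without setting the component's impulse strength.
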(event `self.ReceiveBeginPlay`
  ;[1 1 1] Sets options
  (set `RadialForceComponent.Falloff` (`self.Falloff`) (`self.RadialForce`))
  (set `RadialForceComponent.ForceStrength` (`self.ForceStrength`) (`self.RadialForce`)))

(event `self.ReceiveTick`
  (params (DeltaSeconds :type "Float (single-precision)"))
  (if (`self.Enabled`)
    (`RadialForceComponent.FireImpulse` (`self.RadialForce`))))

(fn `UserConstructionScript`)