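; Earthquake actor that knocks physics objects around with radial impulses while shaking the first player's camera.
; Activate takes a strength, applies it to four RadialForce components, plays CameraShake1 on player controller 0, then fires all four impulses.
; BeginPlay and Tick are empty, and the delayed and random-chance trigger logic is disconnected, so the quake only runs when Activate is called externally.
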(event `self.ReceiveBeginPlay`)

(event `self.ReceiveTick`
  (params (DeltaSeconds :type "Float (single-precision)")))

(fn `Activate`
  (params (Strength :type "Float (double-precision)"))
  (bind _radialforce (`self.RadialForce`))
  (bind _radialforce1 (`self.RadialForce1`))
  (bind _radialforce2 (`self.RadialForce2`))
  (bind _radialforce3 (`self.RadialForce3`))
  (`|ExecutionSequence`
    (:`then_0`
      (`|ExecutionSequence`
        (:`then_0`
          (set `RadialForceComponent.ImpulseStrength` Strength _radialforce))
        (:`then_1`
          (set `RadialForceComponent.ImpulseStrength` Strength _radialforce1))
        (:`then_2`
          (set `RadialForceComponent.ImpulseStrength` Strength _radialforce2))
        (:`then_3`
          (set `RadialForceComponent.ImpulseStrength` Strength _radialforce3))))
    (:`then_1`
      (`PlayerController.ClientStartCameraShake` :`self` (`GameplayStatics.GetPlayerController` 0) :`Shake` "/Game/Blueprints/CameraShake1.CameraShake1_C")
      (`|ExecutionSequence`
        (:`then_0`
          (`RadialForceComponent.FireImpulse` _radialforce))
        (:`then_1`
          (`RadialForceComponent.FireImpulse` _radialforce1))
        (:`then_2`
          (`RadialForceComponent.FireImpulse` _radialforce2))
        (:`then_3`
          (`RadialForceComponent.FireImpulse` _radialforce3))))))

(fn `UserConstructionScript`)