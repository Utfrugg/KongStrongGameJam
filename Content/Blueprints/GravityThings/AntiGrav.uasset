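; AntiGrav periodically toggles gravity off and on for every BP_BaseItem actor in the level.
; Tick starts a three-second delay, then each item's mesh gets a +Y impulse and loses gravity.
; A five-second delay inside that loop leads to re-enabling gravity on all items and looping back.
; D-pad Up handlers only iterate items; gravity and camera-rotation nodes outside the cycle are disconnected.
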(event `self.ReceiveTick`
  (params (DeltaSeconds :type "Float (single-precision)"))
  (`KismetSystemLibrary.Delay` 3.0 :!label _label)
  (bind _outactors (`GameplayStatics.GetAllActorsOfClass` "/Game/Blueprints/ItemSpawner/BP_BaseItem.BP_BaseItem_C"))
  (for _array_element _outactors
    (bind _staticmesh (`/Game/Blueprints/ItemSpawner/BP_BaseItem.StaticMesh` _array_element))
    (`PrimitiveComponent.AddImpulse` _staticmesh (0.0 100.0 0.0) "None" false)
    (`PrimitiveComponent.SetEnableGravity` _staticmesh false)
    (`KismetSystemLibrary.Delay` 5.0)
    (bind _outactors_2 (`GameplayStatics.GetAllActorsOfClass` "/Game/Blueprints/ItemSpawner/BP_BaseItem.BP_BaseItem_C"))
    (for _array_element_2 _outactors_2
      (`PrimitiveComponent.SetEnableGravity` (`/Game/Blueprints/ItemSpawner/BP_BaseItem.StaticMesh` _array_element_2) true)
      (goto _label))))

(event `Key|Gamepad_DPad_Up`
  (params (Key :type "Key Structure"))
  (:`Pressed`
    (bind _outactors (`GameplayStatics.GetAllActorsOfClass` "/Game/Blueprints/ItemSpawner/BP_BaseItem.BP_BaseItem_C"))
    (for _array_element _outactors
      _))
  (:`Released`
    (bind _outactors_2 (`GameplayStatics.GetAllActorsOfClass` "/Game/Blueprints/ItemSpawner/BP_BaseItem.BP_BaseItem_C"))
    (for _array_element_2 _outactors_2
      _)))

(fn `UserConstructionScript`)