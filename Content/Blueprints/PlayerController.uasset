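; Player controller that handles the CatSlap input and forwards it to the possessed BP_SatanCat pawn.
; Pressing prints the current charge as a power percentage, resets and halts charging, then calls CatSlap.
; Releasing calls ReleaseTelekenetics and resumes charging, which Tick fills toward full over TimeToFullyCharge.
; The charge value is only printed, never passed to the pawn.
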(event `self.ReceiveTick`
  (params (DeltaSeconds :type "Float (single-precision)"))
  (if (`self.IsCharging`)
    (set `self.CurrentCharge` (`KismetMathLibrary.FMin` 1.0 (+ (/ DeltaSeconds (`self.TimeToFullyCharge`)) (`self.CurrentCharge`))))))

(event `InputAction|CatSlap`
  (params (Key :type "Key Structure"))
  (:`Pressed`
    (`KismetSystemLibrary.PrintString` (`KismetStringLibrary.Concat_StrStr` "CAT SLAP WITH " (`KismetStringLibrary.Conv_DoubleToString` (* (`self.CurrentCharge`) 100.0)) "% POWER"))
    (set `self.IsCharging` false)
    (set `self.CurrentCharge` 0.0)
    (bind _asbp_satan_cat (cast `/Game/Blueprints/BP_SatanCat` (`self.K2_GetPawn`)))
    (`/Game/Blueprints/BP_SatanCat.CatSlap` _asbp_satan_cat))
  (:`Released`
    (set `self.IsCharging` true)
    (bind _asbp_satan_cat_2 (cast `/Game/Blueprints/BP_SatanCat` (`self.K2_GetPawn`)))
    (`/Game/Blueprints/BP_SatanCat.Release Telekenetics` _asbp_satan_cat_2)))

(fn `UserConstructionScript`)