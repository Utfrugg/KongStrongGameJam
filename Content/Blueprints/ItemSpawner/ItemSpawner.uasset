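; ItemSpawner Blueprint that continuously spawns items at its StaticMesh transform, with a special item after every twenty base items.
; A Delay on Tick throttles spawning to roughly half-second intervals, and a counter chooses between BP_BaseItem and BP_SpecialItem, resetting on the latter.
; Base items enter ActorList, whose oldest entry is destroyed and removed once the new index reaches MaxObjects; special items are untracked.
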(event `self.ReceiveTick`
  (params (DeltaSeconds :type "Float (single-precision)"))
  (bind _actorlist (`self.ActorList`))
  (bind _returnvalue (`SceneComponent.K2_GetComponentToWorld` (`self.StaticMesh`)))
  (bind _output (`|GetArrayItem` _actorlist))
  ;[1 1 1] I am so sorry
  (`KismetSystemLibrary.Delay` 0.5)
  ;[1 1 1] Check if 20 items have spawned
  (if (> (`self.MundaneItemCounter`) 19)
    ;[1 1 1] Spawn Special Item
    (set `self.MundaneItemCounter` 0)
    (`|SpawnActorFromClass` "/Game/Blueprints/ItemSpawner/BP_SpecialItem.BP_SpecialItem_C" _returnvalue "Undefined" "OverrideRootScale" null null)
    (else
      ;[1 1 1] Spawn an item
      (bind _returnvalue_2 (`|SpawnActorFromClass` "/Game/Blueprints/ItemSpawner/BP_BaseItem.BP_BaseItem_C" _returnvalue "Undefined" "OverrideRootScale" null null))
      ;[1 1 1] Add 1 to Counter
      (set `self.MundaneItemCounter` (+ (`self.MundaneItemCounter`) 1))
      (bind _returnvalue_3 (`KismetArrayLibrary.Array_Add` _actorlist _returnvalue_2))
      (`KismetSystemLibrary.PrintString` (`KismetStringLibrary.Conv_IntToString` _returnvalue_3))
      (if (>= _returnvalue_3 (`self.MaxObjects`))
        (`/Engine/EditorBlueprintResources/StandardMacros.IsValid` _output
          (:`Is Valid`
            (`self.K2_DestroyActor` _output))
          (:`Is Not Valid`
            _))
        (`KismetArrayLibrary.Array_Remove` _actorlist)))))

(fn `UserConstructionScript`)