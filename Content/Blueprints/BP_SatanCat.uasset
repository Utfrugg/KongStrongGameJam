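; BP_SatanCat is a controllable cat that grabs nearby static mesh actors with telekinesis and launches them.
; CatSlap collects actors overlapping its sphere and disables their gravity.
; Tick pulls them toward GravitationPoint with damped horizontal impulses, sets their height, draws predicted launch paths and rotates the spring arm from aim axes.
; ReleaseTelekenetics restores gravity, flings them opposite GravitationPoint's forward vector with added lift, and clears the list.
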(event `InputAxis|ForwardBackward`
  (params (AxisValue :type "Float (single-precision)"))
  ;[1 1 1] Movement
  (`self.AddMovementInput` (`KismetMathLibrary.GetForwardVector` (`self.GetControlRotation`)) AxisValue))

(event `InputAxis|LeftRight`
  (params (AxisValue :type "Float (single-precision)"))
  ;[1 1 1] Movement
  (`self.AddControllerYawInput` (* AxisValue 1.5)))

(event `CatSlap`
  ;[1 1 1] Cat slap
  (for _array_element (`PrimitiveComponent.GetOverlappingActors` (`self.Sphere`) null)
    (bind _asstatic_mesh_actor (cast `StaticMeshActor` _array_element))
    (`KismetSystemLibrary.PrintString` (`KismetSystemLibrary.GetDisplayName` _array_element))
    (`KismetArrayLibrary.Array_Add` (`self.TelekinesisedObjects`) _asstatic_mesh_actor)
    (`PrimitiveComponent.SetEnableGravity` (`StaticMeshActor.StaticMeshComponent` _asstatic_mesh_actor) false)))

(event `self.ReceiveTick`
  (params (DeltaSeconds :type "Float (single-precision)"))
  (bind _returnvalue (`self.GetInputAxisKeyValue`))
  (bind _returnvalue_2 (`self.GetInputAxisKeyValue`))
  (bind _launchforcestrength (`self.LaunchForceStrength`))
  (bind _wobbledampening (`self.WobbleDampening`))
  (bind _telekinesisedobjects (`self.TelekinesisedObjects`))
  (bind _returnvalue_3 (`KismetMathLibrary.DegAtan2` (- 0.0 _returnvalue) _returnvalue_2))
  (bind (_returnvalue_x _returnvalue_y) (`KismetMathLibrary.BreakVector` (* (`KismetMathLibrary.NegateVector` (`SceneComponent.GetForwardVector` (`self.gravitation point`))) (`KismetMathLibrary.MakeVector` _launchforcestrength _launchforcestrength))))
  (`|ExecutionSequence`
    (:`then_0`
      ;[1 1 1] Update Telekinesis
      (for _array_element _telekinesisedobjects
        (`/Engine/EditorBlueprintResources/StandardMacros.IsValid` _array_element
          (:`Is Valid`
            (bind _asstatic_mesh_actor (cast `StaticMeshActor` _array_element))
            (bind _returnvalue_4 (`SceneComponent.K2_GetComponentLocation` (`StaticMeshActor.StaticMeshComponent` _asstatic_mesh_actor)))
            (bind (_returnvalue_x_2 _returnvalue_y_2 _returnvalue_z) (`KismetMathLibrary.BreakVector` (- (`SceneComponent.K2_GetComponentLocation` (`self.gravitation point`)) _returnvalue_4)))
            (`PrimitiveComponent.AddImpulse` (`StaticMeshActor.StaticMeshComponent` _asstatic_mesh_actor) (`KismetMathLibrary.MakeVector` (/ _returnvalue_x_2 _wobbledampening) (/ _returnvalue_y_2 _wobbledampening)) "None" true)
            (`self.K2_SetActorLocation` _asstatic_mesh_actor (`KismetMathLibrary.MakeVector` (.x _returnvalue_4) (.y _returnvalue_4) _returnvalue_z) true false)
            ;[0.826 0.06447 1] Debug
            (`GameplayStatics.Blueprint_PredictProjectilePath_ByTraceChannel` _returnvalue_4 (`KismetMathLibrary.MakeVector` (- _returnvalue_x _returnvalue_x_2) (- _returnvalue_y _returnvalue_y_2) (`self.LaunchHeightStrength`)) true 0.0 "ECC_WorldDynamic" false (`|MakeArray` _asstatic_mesh_actor :!type "Actor Object Reference") "ForDuration"))
          (:`Is Not Valid`
            (`KismetArrayLibrary.Array_RemoveItem` _telekinesisedobjects _array_element)))))
    (:`then_1`
      ;[1 1 1] Aiming
      (if (not (and (== _returnvalue 0.0) (== _returnvalue_2 0.0)))
        (`KismetSystemLibrary.PrintString` (`KismetStringLibrary.Conv_DoubleToString` _returnvalue_3) true true (struct :`R` 1.0 :`G` 0.091998 :`A` 1.0) 0.0)
        (`SceneComponent.K2_SetWorldRotation` (`self.SpringArm`) (`KismetMathLibrary.MakeRotator` 0.0 0.0 _returnvalue_3) false false)))
    (:`then_2`)))

(event `Release Telekenetics`
  (bind _telekinesisedobjects (`self.TelekinesisedObjects`))
  (bind _launchforcestrength (`self.LaunchForceStrength`))
  (bind (_returnvalue_x _returnvalue_y) (`KismetMathLibrary.BreakVector` (* (`KismetMathLibrary.NegateVector` (`SceneComponent.GetForwardVector` (`self.gravitation point`))) (`KismetMathLibrary.MakeVector` _launchforcestrength _launchforcestrength))))
  ;[1 1 1] Update Telekinesis
  (for _array_element _telekinesisedobjects
    (`/Engine/EditorBlueprintResources/StandardMacros.IsValid` _array_element
      (:`Is Valid`
        (bind _asstatic_mesh_actor (cast `StaticMeshActor` _array_element))
        (bind _staticmeshcomponent (`StaticMeshActor.StaticMeshComponent` _asstatic_mesh_actor))
        (`PrimitiveComponent.SetEnableGravity` _staticmeshcomponent true)
        (bind (_returnvalue_x_2 _returnvalue_y_2) (`KismetMathLibrary.BreakVector` (`self.GetVelocity` _asstatic_mesh_actor)))
        (`PrimitiveComponent.SetPhysicsLinearVelocity` (`StaticMeshActor.StaticMeshComponent` _asstatic_mesh_actor) (`KismetMathLibrary.MakeVector` _returnvalue_x_2 _returnvalue_y_2) false "None")
        (`PrimitiveComponent.AddImpulse` _staticmeshcomponent (`KismetMathLibrary.MakeVector` _returnvalue_x _returnvalue_y (`self.LaunchHeightStrength`)) "None" true))))
  (`KismetArrayLibrary.Array_Clear` _telekinesisedobjects))

(fn `UserConstructionScript`)